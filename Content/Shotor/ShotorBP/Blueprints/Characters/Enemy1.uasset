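; Enemy character that chases pawns it senses, takes projectile damage and destroys itself when health runs out.
; Pawn sensing drives a simple move-to-actor, with the noise event reusing the seen-pawn target instead of the noise source.
; Body hits from FirstPersonProjectile subtract its damage through UpdateHealth, which destroys the actor below zero or updates HealthPercent.
; On BeginPlay it passes itself to its HealthBar widget.
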(event `self.PawnSensing.OnSeePawn`
  (params (Pawn :type "Pawn Object Reference"))
  ;[1 1 1] Vision and noise detection
  (`AIBlueprintHelperLibrary.SimpleMoveToActor` (`self.GetController`) Pawn :!label _label))

(event `self.PawnSensing.OnHearNoise`
  (params (Instigator :type "Pawn Object Reference") (Location :type "Vector Structure (by ref)") (Volume :type "Float (single-precision)"))
  ;[1 1 1] Vision and noise detection
  (goto _label))

(event `self.BodyCollision.OnComponentHit`
  (params (HitComponent :type "PrimitiveComponent Object Reference") (OtherActor :type "Actor Object Reference") (OtherComp :type "PrimitiveComponent Object Reference") (NormalImpulse :type "Vector Structure") (Hit :type "HitResult Structure (by ref)"))
  (bind _asfirst_person_projectile (cast `/Game/Shotor/ShotorBP/Blueprints/FirstPersonProjectile` OtherActor))
  (`self.updateHealth` (- (`self.health`) (`/Game/Shotor/ShotorBP/Blueprints/FirstPersonProjectile.Damage` _asfirst_person_projectile))))

(event `self.ReceiveBeginPlay`
  (bind _ashealth_bar (cast `/Game/Shotor/ShotorBP/Menu/UI/HealthBar` (`WidgetComponent.GetUserWidgetObject` (`self.HealthBar`))))
  (set `/Game/Shotor/ShotorBP/Menu/UI/HealthBar.Enemy` self _ashealth_bar))

(fn `updateHealth`
  (params (healthUpdate :type "Float (double-precision)"))
  (bind _output_get (set `self.health` healthUpdate))
  (if (< _output_get 0.0)
    ;[1 1 1] Dead
    (`self.K2_DestroyActor`)
    (else
      ;[1 1 1] Alive
      (set `self.healthPercent` (/ (`self.health`) (`self.maxHealth`))))))

(fn `UserConstructionScript`)